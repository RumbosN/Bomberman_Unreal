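; BP_Grabbable_Statue is a physics statue prop that can be picked up and released by a grabbing component.
; On Grabbed, it disables physics and collision and attaches its static mesh to the grabber, keeping its world transform.
; On Dropped, it re-enables physics and collision, detaches, and copies the releasing component's linear and angular velocity onto the mesh so it can be thrown.
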(event EventGrabbed
  (params (Grabbed%20By :type Scene%20Component%20Object%20Reference))
  (bind _staticmeshcomponent (Variables|Debug|GetStaticMeshComponent))
  (Physics|SetSimulatePhysics _staticmeshcomponent false)
  (Transformation|AttachComponentToComponent _staticmeshcomponent Grabbed%20By "None" "KeepWorld" "KeepWorld" "KeepWorld" false)
  (Collision|SetCollisionEnabled (Variables|Debug|GetStaticMeshComponent) "NoCollision"))

(event EventDropped
  (params (Dropped%20By :type Static%20Mesh%20Component%20Object%20Reference))
  (bind _staticmeshcomponent (Variables|Debug|GetStaticMeshComponent))
  (bind _staticmeshcomponent_2 (Variables|Debug|GetStaticMeshComponent))
  (Physics|SetSimulatePhysics _staticmeshcomponent true)
  (Transformation|DetachFromActor "KeepWorld" "KeepWorld" "KeepWorld")
  (Collision|SetCollisionEnabled _staticmeshcomponent "QueryAndPhysics")
  (bind _returnvalue (Physics|GetPhysicsLinearVelocity Dropped%20By "None"))
  (Physics|SetPhysicsLinearVelocity _staticmeshcomponent_2 _returnvalue false "None")
  (Class|PrimitiveComponent|SetPhysicsAngularVelocityinDegrees _staticmeshcomponent_2 (Physics|GetPhysicsAngularVelocityinDegrees Dropped%20By "None") false "None"))

(fn ConstructionScript)