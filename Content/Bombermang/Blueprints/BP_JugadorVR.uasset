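; VR player pawn for a bomb-placing game, with camera-relative movement, axis-driven turning, jumping and teleporting.
; While alive, Tick moves the pawn, eases mesh rotation toward travel and pulses haptics on hands overlapping IGrabbable actors, which can be grabbed and dropped.
; Held inputs trace from each hand; release teleports with a camera fade (right) or spawns a capped bomb (left).
; DestroyMySelf decrements lives, opening Game_Over with the score when none remain.
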(event EventBeginPlay)

(event EventDestroyMySelf
  (bind _result (Math|Integer|DecrementInt (Variables|Default|GetLives))
    (:%20%20
      (if (<= _result 0)
        (Variables|Default|SetIsAlive false)
        (Utilities|FlowControl|Delay 1.0)
        (Viewport|RemoveAllWidgets)
        (Game|OpenLevel(byName) "Game_Over" true (Utilities|String|Append "points=" (Utilities|String|ToString(Integer) (Variables|Default|GetScore))))))))

(event EventTick
  (params (DeltaSeconds :type Float%20%28single-precision%29))
  (if (Variables|Default|GetIsAlive)
    (CallFunction|SetMovement DeltaSeconds)
    (CallFunction|SetRotation)
    (CallFunction|SetHaptics "Left")
    (CallFunction|SetHaptics "Right")
    (Utilities|FlowControl|Sequence
      (:then_0
        (if (Variables|Default|GetTeleportPressed)
          (CallFunction|LineTrace "Right" (Variables|Default|GetTeleport%20Obj%20Type) (Math|Color|MakeColor 252 7 3))))
      (:then_1
        (if (Variables|Default|GetPutBombPressed)
          (CallFunction|LineTrace "Left" (Variables|Default|GetLaser%20Object%20Types) (Math|Color|MakeColor 3 3 252)))))
    (else
      (Rendering|SetVisibility (Variables|Default|GetHUD) false false))))

(event Input|ActionEvents|InputActionGrabL
  (params (Key :type Key%20Structure :default "None"))
  (:Pressed
    (CallFunction|Grab "Left"))
  (:Released
    (CallFunction|Drop "Left")))

(event Input|ActionEvents|InputActionGrabR
  (params (Key :type Key%20Structure :default "None"))
  (:Pressed
    (CallFunction|Grab "Right"))
  (:Released
    (CallFunction|Drop "Right")))

(event Input|ActionEvents|InputActionTeleport
  (params (Key :type Key%20Structure :default "None"))
  (bind _returnvalue (Game|GetPlayerCameraManager 0))
  (bind _hit_point (Variables|Default|GetHit%20Point))
  (bind (_bblockinghit _binitialoverlap _time _distance _location _impactpoint _normal _impactnormal _physmat _hitactor) (Collision|BreakHitResult _hit_point))
  (:Pressed
    (Variables|Default|SetTeleportPressed true))
  (:Released
    (if (Variables|Default|GetIsAlive)
      (Variables|Default|SetTeleportPressed false)
      (if (!= _hitactor 0)
        (CameraFades|StartCameraFade :self _returnvalue :ToAlpha 1.0 :Duration 0.5)
        (Transformation|SetActorLocation (+ _impactpoint (* _impactnormal 1e+02)) false false)
        (Timeline|Wait Play
          (:Finished
            (CameraFades|StartCameraFade :self _returnvalue :FromAlpha 1.0 :Duration 0.5)))))))

(event Input|ActionEvents|InputActionJump
  (params (Key :type Key%20Structure :default "None"))
  (:Pressed
    (if (and (> (Utilities|Array|Length (Collision|GetOverlappingActors (Variables|Default|GetGround%20Detector) 0 :!class /Script/Engine.PrimitiveComponent)) 1) (Variables|Default|GetIsAlive))
      (Physics|AddImpulse (Variables|Default|GetCapsule) "0, 0,400.000000" "None" true))))

(event Input|ActionEvents|InputActionPutBomb
  (params (Key :type Key%20Structure :default "None"))
  (bind _hit_object (Variables|Default|GetHit%20Object))
  (bind (_bblockinghit _binitialoverlap _time _distance _location _impactpoint _normal _impactnormal _physmat _hitactor) (Collision|BreakHitResult _hit_object))
  (:Pressed
    (Variables|Default|SetPutBombPressed true))
  (:Released
    (if (Variables|Default|GetIsAlive)
      (Variables|Default|SetPutBombPressed false)
      (if (and (!= _hitactor 0) (!= (Variables|Default|GetBombas) (Variables|Default|GetMaxBombas)))
        (Game|SpawnActorfromClass "/Game/Bombermang/Blueprints/BP_Bomb.BP_Bomb_C" (Math|Transform|MakeTransform (+ _impactpoint (* _impactnormal 5e+01))) "AdjustIfPossibleButAlwaysSpawn" 0 0)
        (Math|Integer|IncrementInt (Variables|Default|GetBombas))))))

(event Input|AxisEvents|InputAxisMoveForward
  (params (AxisValue :type Float%20%28single-precision%29))
  (bind _camera (Variables|Default|GetCamera))
  (bind _returnvalue (Math|Vector|GetForwardVector _camera))
  (bind (_x _y) (Math|Vector|BreakVector _returnvalue))
  (Pawn|Input|AddMovementInput (Math|Vector|MakeVector _x _y 0.0) AxisValue false))

(event Input|AxisEvents|InputAxisMoveRight
  (params (AxisValue :type Float%20%28single-precision%29))
  (bind _camera (Variables|Default|GetCamera))
  (bind _returnvalue (Math|Vector|GetRightVector _camera))
  (bind (_x _y) (Math|Vector|BreakVector _returnvalue))
  (Pawn|Input|AddMovementInput (Math|Vector|MakeVector _x _y 0.0) AxisValue false))

(event Input|AxisEvents|InputAxisRotation
  (params (AxisValue :type Float%20%28single-precision%29))
  (CallFunction|SetCameraRotation AxisValue))

(fn ConstructionScript)

(fn SetMovement
  (params (Delta%20Seconds :type Float%20%28single-precision%29))
  (bind _returnvalue (Class|Pawn|ConsumeMovementInputVector))
  (Variables|Default|SetMovement (Math|Vector|Normalize _returnvalue))
  (Transformation|AddActorLocalOffset (* (Math|Vector|Normalize _returnvalue) (* (Variables|Default|GetSpeed) Delta%20Seconds)) false false)
  (Variables|Default|SetCurrent%20Speed (Math|Vector|VectorLength (* (Math|Vector|Normalize _returnvalue) (* (Variables|Default|GetSpeed) Delta%20Seconds)))))

(fn SetRotation
  (bind _returnvalue (Transformation|GetActorLocation))
  (bind _movement (Variables|Default|GetMovement))
  (bind _skeletalmesh (Variables|Default|GetSkeletalMesh))
  (bind _rotation_offset (Variables|Default|GetRotation%20Offset))
  (bind (_roll _pitch _yaw) (Math|Rotator|BreakRotator _rotation_offset))
  (bind _returnvalue_2 (+ _returnvalue _movement))
  (bind _returnvalue_3 (Math|Rotator|FindLookatRotation _returnvalue _returnvalue_2))
  (bind _returnvalue_4 (Math|Vector|MakeVector _roll _pitch _yaw))
  (bind (_roll_2 _pitch_2 _yaw_2) (Math|Rotator|BreakRotator _returnvalue_3))
  (bind _returnvalue_5 (Math|Vector|MakeVector _roll_2 _pitch_2 _yaw_2))
  (bind _returnvalue_6 (+ _returnvalue_5 _returnvalue_4))
  (bind (_x _y _z) (Math|Vector|BreakVector _returnvalue_6))
  (if (> (Math|Vector|VectorLength (Variables|Default|GetMovement)) 0.0)
    (Transformation|SetRelativeRotation _skeletalmesh (Math|Interpolation|RInterpTo (Variables|/Script/Engine.SceneComponent|GetRelativeRotation _skeletalmesh) (Math|Rotator|MakeRotator _x _y _z) (Utilities|Time|GetWorldDeltaSeconds) 5.0) false false)))

(fn Grab
  (params (Hand :type EControllerHand%20Enum :default "Left"))
  (bind _returnvalue (Utilities|Enum|Equal(Enum) Hand "Left"))
  (Utilities|FlowControl|Sequence
    (:then_0
      (if _returnvalue
        (LocalVariables|SetCurrent%20Hand (Variables|Default|GetHand%20L))
        (else
          (LocalVariables|SetCurrent%20Hand (Variables|Default|GetHand%20R)))))
    (:then_1
      (bind _array_element (Utilities|Array|ForEachLoopwithBreak (Collision|GetOverlappingActors (LocalVariables|GetCurrent%20Hand) 0 :!class /Script/Engine.PrimitiveComponent))
        (:LoopBody
          (bind _asigrabbable (Utilities|Casting|CastToIGrabbable _array_element))
          (if _returnvalue
            (Variables|Default|SetGrabbed%20L _asigrabbable)
            (else
              (Variables|Default|SetGrabbed%20R _asigrabbable)))
          (Default|Grabbed _asigrabbable (LocalVariables|GetCurrent%20Hand))
          (Rendering|Material|SetMaterial (LocalVariables|GetCurrent%20Hand) 0 (Variables|Default|GetAlternative%20Material)))))))

(fn Drop
  (params (Hand :type EControllerHand%20Enum :default "Left"))
  (bind _hand_l (Variables|Default|GetHand%20L))
  (bind _hand_r (Variables|Default|GetHand%20R))
  (bind _default_material (Variables|Default|GetDefault%20Material))
  (if (Utilities|Enum|Equal(Enum) Hand "Left")
    (if (not (== (Utilities|ToObject(Interface) (Variables|Default|GetGrabbed%20L)) 0))
      (Default|Dropped (Variables|Default|GetGrabbed%20L) _hand_l)
      (Variables|Default|SetGrabbed%20L 0)
      (Rendering|Material|SetMaterial _hand_l 0 _default_material))
    (elif (not (== (Utilities|ToObject(Interface) (Variables|Default|GetGrabbed%20R)) 0))
      (Default|Dropped (Variables|Default|GetGrabbed%20R) _hand_r)
      (Variables|Default|SetGrabbed%20R 0)
      (Rendering|Material|SetMaterial _hand_r 0 _default_material))))

(fn SetHaptics
  (params (Hand :type EControllerHand%20Enum :default "Left"))
  (bind _returnvalue (Game|GetPlayerController 0))
  (Utilities|FlowControl|Sequence
    (:then_0
      (if (Utilities|Enum|Equal(Enum) Hand "Left")
        (LocalVariables|SetHand%20Mesh (Variables|Default|GetHand%20L))
        (else
          (LocalVariables|SetHand%20Mesh (Variables|Default|GetHand%20R)))))
    (:then_1
      (for _array_element (Collision|GetOverlappingActors (LocalVariables|GetHand%20Mesh) 0 :!class /Script/Engine.PrimitiveComponent)
        (Utilities|Casting|CastToIGrabbable _array_element)
        (Math|Integer|IncrementInt (LocalVariables|GetOverlaps))))
    (:then_2
      (if (> (LocalVariables|GetOverlaps) 0)
        (Class|PlayerController|SetHapticsbyValue _returnvalue 1.0 1.0 Hand)
        (else
          (Class|PlayerController|SetHapticsbyValue _returnvalue 0.0 0.0 Hand))))))

(fn LineTrace
  (params (Hand :type EControllerHand%20Enum :default "Left") (ObjectType :type Array%20of%20EObjectTypeQuery%20Enums :default "ObjectTypeQuery1") (Color :type Color%20Structure))
  (bind _returnvalue (Utilities|Enum|Equal(Enum) Hand "Left"))
  (Utilities|FlowControl|Sequence
    (:then_0
      (if _returnvalue
        (LocalVariables|SetHand%20Obj (Variables|Default|GetHand%20L))
        (else
          (LocalVariables|SetHand%20Obj (Variables|Default|GetHand%20R)))))
    (:then_1
      (bind _outhit (Collision|LineTraceForObjects (Transformation|GetWorldLocation (LocalVariables|GetHand%20Obj)) (+ (Transformation|GetWorldLocation (LocalVariables|GetHand%20Obj)) (* (Math|Vector|GetUpVector (LocalVariables|GetHand%20Obj)) 1e+03)) ObjectType false 0 "ForOneFrame" true (Math|Conversions|ToLinearColor(Color) Color)))
      (if _returnvalue
        (Variables|Default|SetHit%20Object _outhit)
        (else
          (Variables|Default|SetHit%20Point _outhit))))))

(fn SetCameraRotation
  (params (Axis%20Value :type Float%20%28single-precision%29))
  (bind _vr_root (Variables|Default|GetVR%20Root))
  (bind _returnvalue (Transformation|GetWorldRotation _vr_root))
  (bind (_roll _pitch _yaw) (Math|Rotator|BreakRotator _returnvalue))
  (Transformation|SetWorldRotation (Variables|Default|GetVR%20Root) (Math|Rotator|MakeRotator _roll _pitch (+ _yaw (* Axis%20Value 5.0))) false true))