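; BP_Rock is a rock actor in Bombermang that moves up and down continuously from where it is placed.
; On BeginPlay it stores its initial location and starts a timeline, whose value scales a configurable Z distance in centimeters to offset the rock with swept movement.
; When the timeline finishes it flips direction, producing an endless ping-pong motion without using Tick.
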(event EventBeginPlay
  (Variables|Default|SetPosición%20Inicial (Transformation|GetActorLocation))
  (bind (_direction _valor) (Timeline|Timeline_0 Play)
    (:Update
      (Transformation|SetActorLocation (+ (Math|Vector|MakeVector 0.0 0.0 (* _valor (Variables|Default|GetDesplazamiento%20en%20Z%20%28cm%29))) (Variables|Default|GetPosición%20Inicial)) true false))
    (:Finished
      (if (Utilities|Enum|Equal(Enum) _direction "Forward")
        (Timeline|Timeline_0 ReverseFromEnd)
        (else
          (Timeline|Timeline_0 PlayFromStart))))))

(fn ConstructionScript)