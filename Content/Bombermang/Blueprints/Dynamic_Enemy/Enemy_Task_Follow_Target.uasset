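; Behavior tree task for a dynamic Bombermang enemy that moves its pawn toward the target actor stored in the blackboard.
; On execute it calls AI MoveTo with a fixed acceptance radius and writes a moving speed to a blackboard float.
; When the move succeeds or fails, it finishes with the matching result and resets that speed to zero.
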(event EventReceiveExecuteAI
  (params (OwnerController :type AI%20Controller%20Object%20Reference) (ControlledPawn :type Pawn%20Object%20Reference))
  (AI|AIMoveTo ControlledPawn "0, 0, 0" (AI|BehaviorTree|GetBlackboardValueasActor (Variables|Default|GetBB%20Target%20Key)) 1.5e+02 false
    (:then
      (Class|BTFunctionLibrary|SetBlackboardValueasFloat (Variables|Default|GetBB%20Speed%20Key) 3.0))
    (:OnSuccess
      (AI|BehaviorTree|FinishExecute true)
      (Class|BTFunctionLibrary|SetBlackboardValueasFloat (Variables|Default|GetBB%20Speed%20Key) 0.0))
    (:OnFail
      (AI|BehaviorTree|FinishExecute false)
      (Class|BTFunctionLibrary|SetBlackboardValueasFloat (Variables|Default|GetBB%20Speed%20Key) 0.0))))