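; Player pawn Blueprint that moves from forward/right axis input and turns its skeletal mesh toward the direction of travel.
; Each Tick it consumes and normalizes the input vector, applies a speed-scaled local offset without sweep, and stores that step's length as CurrentSpeed.
; The mesh interpolates toward the movement's look-at rotation plus RotationOffset.
; Tick also increments Score every frame and prints raw input for debugging.
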(event EventBeginPlay)

(event EventTick
  (params (DeltaSeconds :type Float%20%28single-precision%29))
  (CallFunction|SetMovement DeltaSeconds)
  (CallFunction|SetRotation)
  (bind _result (Math|Integer|IncrementInt (Variables|Default|GetScore))
    (:%20%20
      (Variables|Default|SetScore _result))))

(event Input|AxisEvents|InputAxisMoveForward
  (params (AxisValue :type Float%20%28single-precision%29))
  (Pawn|Input|AddMovementInput (Transformation|GetActorForwardVector) AxisValue false))

(event Input|AxisEvents|InputAxisMoveRight
  (params (AxisValue :type Float%20%28single-precision%29))
  (Pawn|Input|AddMovementInput (Transformation|GetActorRightVector) AxisValue false))

(fn ConstructionScript)

(fn SetMovement
  (params (Delta%20Seconds :type Float%20%28single-precision%29))
  (bind _returnvalue (Class|Pawn|ConsumeMovementInputVector))
  (Development|PrintString (Utilities|String|ToString(Vector) _returnvalue))
  (Variables|Default|SetMovement (Math|Vector|Normalize _returnvalue))
  (Transformation|AddActorLocalOffset (* (Math|Vector|Normalize _returnvalue) (* (Variables|Default|GetSpeed) Delta%20Seconds)) false false)
  (Variables|Default|SetCurrent%20Speed (Math|Vector|VectorLength (* (Math|Vector|Normalize _returnvalue) (* (Variables|Default|GetSpeed) Delta%20Seconds)))))

(fn SetRotation
  (bind _returnvalue (Transformation|GetActorLocation))
  (bind _movement (Variables|Default|GetMovement))
  (bind _skeletalmesh (Variables|Default|GetSkeletalMesh))
  (bind _rotation_offset (Variables|Default|GetRotation%20Offset))
  (bind (_roll _pitch _yaw) (Math|Rotator|BreakRotator _rotation_offset))
  (bind _returnvalue_2 (+ _returnvalue _movement))
  (bind _returnvalue_3 (Math|Rotator|FindLookatRotation _returnvalue _returnvalue_2))
  (bind _returnvalue_4 (Math|Vector|MakeVector _roll _pitch _yaw))
  (bind (_roll_2 _pitch_2 _yaw_2) (Math|Rotator|BreakRotator _returnvalue_3))
  (bind _returnvalue_5 (Math|Vector|MakeVector _roll_2 _pitch_2 _yaw_2))
  (bind _returnvalue_6 (+ _returnvalue_5 _returnvalue_4))
  (bind (_x _y _z) (Math|Vector|BreakVector _returnvalue_6))
  (if (> (Math|Vector|VectorLength (Variables|Default|GetMovement)) 0.0)
    (Transformation|SetRelativeRotation _skeletalmesh (Math|Interpolation|RInterpTo (Variables|/Script/Engine.SceneComponent|GetRelativeRotation _skeletalmesh) (Math|Rotator|MakeRotator _x _y _z) (Utilities|Time|GetWorldDeltaSeconds) 5.0) false false)))